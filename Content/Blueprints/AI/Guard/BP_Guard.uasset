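; Guard AI that patrols and reacts to the player through pawn sensing.
; BeginPlay sets Patrol to true before branching on it, so the guard always enters PatrolState rather than IdleState.
; Seeing BP_Player fires GameOver, which sets WasSeen on the player pawn, then calls AlertState.
; Hearing a noise passes its instigator and location to SuspiciousState at fixed volume; the state functions are defined outside these graphs.
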(event `self.ReceiveBeginPlay`
  ;[1 1 1] Change between beginning idle state or patroling state
  (bind _output_get (set `self.bPatrol` true))
  (if _output_get
    (`self.PatrolState`)
    (else
      (`self.IdleState`))))

(event `GameOver`
  ;[1 1 1] Set the was seen boolean
  (bind _asbp_player (cast `/Game/Blueprints/Player/BP_Player` (`GameplayStatics.GetPlayerPawn` 0)))
  (set `FPSCharacter.bWasSeen` true _asbp_player))

(event `self.PawnSensingComp.OnSeePawn`
  (params (Pawn :type "Pawn Object Reference"))
  ;[1 1 1] Checks if the player was seen, if so call the audio event and game over event
  (bind _asbp_player (cast `/Game/Blueprints/Player/BP_Player` Pawn))
  (`self.GameOver`)
  (`self.AlertState` _asbp_player))

(event `self.PawnSensingComp.OnHearNoise`
  (params (Instigator :type "Pawn Object Reference") (Location :type "Vector Structure (by ref)") (Volume :type "Float (single-precision)"))
  ;[1 1 1] Pawn Sensing no longer works in C++ so here is the pawn being distracted Then rotate back after 3 seconds
  (`self.SuspiciousState` Instigator Location 1.0))

(fn `UserConstructionScript`)